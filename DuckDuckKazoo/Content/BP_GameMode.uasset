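; Game mode for a ducks-versus-hunters match that handles spawning and checks win conditions.
; After a delayed PostLogin, it possesses each new player into a duck at a random spawner and spawns a behavior-tree AI seeker at a random seeker spawner.
; Tick casts player pawn 0 to seeker and duck, printing a win message when its Roasts or Berries count equals three.
; Only that pawn is checked, not the AI seekers.
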(event `self.ReceiveTick`
  (params (DeltaSeconds :type "Float (single-precision)"))
  ;[1 1 1] Win conditions
  (`|ExecutionSequence`
    (:`then_0`
      (bind _asbp_seeker (cast `/Game/TheSeeker/BP_Seeker` (`GameplayStatics.GetPlayerPawn` 0)))
      (bind _output_get (set `self.Hunter` _asbp_seeker))
      (if (== (`/Game/TheSeeker/BP_Seeker.Roasts` _output_get) 3)
        (`KismetSystemLibrary.PrintString` "Hunters win!" true true (struct :`R` 1.0 :`G` 0.464954 :`A` 1.0))))
    (:`then_1`
      (bind _asbp_duck (cast `/Game/Duck/BP_Duck` (`GameplayStatics.GetPlayerPawn` 0)))
      (bind _output_get_2 (set `self.Duck` _asbp_duck))
      (if (== (`/Game/Duck/BP_Duck.Berries` _output_get_2) 3)
        (`KismetSystemLibrary.PrintString` "Ducks win!" true true (struct :`G` 1.0 :`B` 0.180251 :`A` 1.0))))))

(event `self.K2_PostLogin`
  (params (NewPlayer :type "PlayerController Object Reference"))
  ;[1 1 1] Player and hunter spawning logic
  (`KismetSystemLibrary.Delay` 8.0)
  (bind _outactors (`GameplayStatics.GetAllActorsOfClass` "/Game/Map/BP_Spawner.BP_Spawner_C"))
  (bind _output_get (set `self.Out Actors_0` _outactors))
  (bind _returnvalue (`|SpawnActorFromClass` "/Game/Duck/BP_Duck.BP_Duck_C" (`KismetMathLibrary.Conv_VectorToTransform` (`self.K2_GetActorLocation` (`KismetArrayLibrary.Array_Random` _output_get))) "Undefined" "MultiplyWithRoot" null null))
  (`Controller.UnPossess` NewPlayer)
  (`Controller.Possess` NewPlayer _returnvalue)
  (bind _outactors_2 (`GameplayStatics.GetAllActorsOfClass` "/Game/Map/BP_SeekerrSpawner.BP_SeekerrSpawner_C"))
  (bind _output_get_2 (set `self.Out Actors` _outactors_2))
  (bind _outitem (`KismetArrayLibrary.Array_Random` _output_get_2))
  (`AIBlueprintHelperLibrary.SpawnAIFromClass` "/Game/TheSeeker/BP_Seeker.BP_Seeker_C" "/Game/TheSeeker/BT_Seeker.BT_Seeker" (`self.K2_GetActorLocation` _outitem) (`self.K2_GetActorRotation` _outitem) false null))

(fn `UserConstructionScript`)